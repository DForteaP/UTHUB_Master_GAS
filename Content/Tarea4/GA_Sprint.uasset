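; GA_Sprint is a Gameplay Ability that gives the top-down character a short sprint burst when it is moving and not already sprinting.
; Activation sets the Sprinting flag, applies GE_Sprint to self, adds non-replicated loose gameplay tags and launches the character along its amplified horizontal velocity.
; After a fixed delay it clears the flag and tags and ends, while a failed check ends it immediately.
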(event `self.K2_ActivateAbility`
  (bind _returnvalue (`self.GetAbilitySystemComponentFromActorInfo`))
  (bind _character (`self.Character`))
  (bind (_returnvalue_x _returnvalue_y) (`KismetMathLibrary.BreakVector` (* (`Actor.GetVelocity` _character) 5.0)))
  (`self.GetCharacter`)
  (bind _cansprint (`self.CanSprint?`))
  (if _cansprint
    (set `/Game/TopDown/Blueprints/BP_TopDownCharacter.Sprinting?` true (`self.Character`))
    (`AbilitySystemComponent.BP_ApplyGameplayEffectSpecToSelf` _returnvalue (`AbilitySystemComponent.MakeOutgoingSpec` _returnvalue "/Game/Tarea4/GE_Sprint.GE_Sprint_C" 0.0 (`AbilitySystemComponent.MakeEffectContext` _returnvalue)))
    (`AbilitySystemBlueprintLibrary.AddLooseGameplayTags` _character (`self.Gameplay Tags`))
    (`Character.LaunchCharacter` _character (`KismetMathLibrary.MakeVector` _returnvalue_x _returnvalue_y) false false)
    (`KismetSystemLibrary.Delay` 2.0)
    (set `/Game/TopDown/Blueprints/BP_TopDownCharacter.Sprinting?` false (`self.Character`))
    (`AbilitySystemBlueprintLibrary.RemoveLooseGameplayTags` (`self.Character`) (`self.Gameplay Tags`))
    (`self.K2_EndAbility`)
    (else
      (`self.K2_EndAbility`))))

(fn `CanSprint?`
  (returns (CanSprint :type Boolean))
  (return (and (not (`KismetMathLibrary.EqualExactly_VectorVector` (`Actor.GetVelocity` (`self.Character`)))) (not (`/Game/TopDown/Blueprints/BP_TopDownCharacter.Sprinting?` (`self.Character`))))))

(fn `GetCharacter`
  (bind _asbp_top_down_character (cast `/Game/TopDown/Blueprints/BP_TopDownCharacter` (`self.GetAvatarActorFromActorInfo`)))
  (set `self.Character` _asbp_top_down_character))