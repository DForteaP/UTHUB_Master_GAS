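; GA_Attack is a Gameplay Ability that deals a melee-style hit to a pawn in front of its avatar.
; A zero-length sphere trace, offset forward by Range, finds one target and applies GE_Damaged through its Ability System Component.
; Only a valid hit plays the attack montage, disabling movement until completion restores walking and ends the ability.
; A miss ends it immediately, while montage interruption or cancellation has no handler.
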(event `self.K2_ActivateAbility`
  (bind _returnvalue (`self.GetAvatarActorFromActorInfo`))
  (bind _returnvalue_2 (`self.GetAbilitySystemComponentFromActorInfo`))
  (bind _returnvalue_3 (`Actor.GetComponentByClass` (`self.GetAvatarActorFromActorInfo`) "/Script/Engine.CharacterMovementComponent"))
  (bind _returnvalue_4 (+ (`Actor.K2_GetActorLocation` _returnvalue) (* (`Actor.GetActorForwardVector` _returnvalue) (`self.Range`))))
  (bind (_outhit _returnvalue_5) (`KismetSystemLibrary.SphereTraceSingleForObjects` _returnvalue_4 _returnvalue_4 (`self.Range`) (`|MakeArray` "ObjectTypeQuery3" :!type "EObjectTypeQuery Enum") false (`|MakeArray` (`self.GetAvatarActorFromActorInfo`)) "ForDuration"))
  (if _returnvalue_5
    (bind _returnvalue_6 (`Actor.GetComponentByClass` (`.HitActor` (`GameplayStatics.BreakHitResult` _outhit)) "/Script/GameplayAbilities.AbilitySystemComponent"))
    (if (`KismetSystemLibrary.IsValid` _returnvalue_6)
      (`AbilitySystemComponent.BP_ApplyGameplayEffectSpecToTarget` _returnvalue_2 (`AbilitySystemComponent.MakeOutgoingSpec` _returnvalue_2 "/Game/Tarea4/GE_Damaged.GE_Damaged_C" 0.0 (`AbilitySystemComponent.MakeEffectContext` _returnvalue_2)) _returnvalue_6)
      (`AbilityTask_PlayMontageAndWait.CreatePlayMontageAndWaitProxy` "None" (`self.Animation`)
        (:`then`
          (`CharacterMovementComponent.DisableMovement` _returnvalue_3))
        (:`OnCompleted`
          (`CharacterMovementComponent.SetMovementMode` _returnvalue_3 "MOVE_Walking" 0)
          (`self.K2_EndAbility`)))
      (else
        (`self.K2_EndAbility`)))
    (else
      (`self.K2_EndAbility`))))