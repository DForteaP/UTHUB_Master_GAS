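; GA_Guard is a Gameplay Ability that makes the BP_TopDownCharacter perform a guard action.
; On activation it applies the GE_Guard effect to itself, adds loose gameplay tags and plays a montage while disabling movement.
; When the montage completes, it restores walking, removes the tags and ends the ability; interruption or cancellation of the montage has no cleanup handler.
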(event `self.K2_ActivateAbility`
  (bind _returnvalue (`self.GetAbilitySystemComponentFromActorInfo`))
  (bind _returnvalue_2 (`Actor.GetComponentByClass` (`self.GetAvatarActorFromActorInfo`) "/Script/Engine.CharacterMovementComponent"))
  (bind _asbp_top_down_character (cast `/Game/TopDown/Blueprints/BP_TopDownCharacter` (`self.GetAvatarActorFromActorInfo`)))
  (set `self.Character` _asbp_top_down_character)
  (`AbilitySystemComponent.BP_ApplyGameplayEffectSpecToSelf` _returnvalue (`AbilitySystemComponent.MakeOutgoingSpec` _returnvalue "/Game/Tarea4/GE_Guard.GE_Guard_C" 0.0 (`AbilitySystemComponent.MakeEffectContext` _returnvalue)))
  (`AbilitySystemBlueprintLibrary.AddLooseGameplayTags` (`self.Character`) (`self.Gameplay Tags`))
  (`AbilityTask_PlayMontageAndWait.CreatePlayMontageAndWaitProxy` "None" (`self.Animation`) 1.0 "None" true 1.0 0.0 true
    (:`then`
      (`CharacterMovementComponent.DisableMovement` _returnvalue_2))
    (:`OnCompleted`
      (`CharacterMovementComponent.SetMovementMode` _returnvalue_2 "MOVE_Walking" 0)
      (`AbilitySystemBlueprintLibrary.RemoveLooseGameplayTags` (`self.Character`) (`self.Gameplay Tags`))
      (`self.K2_EndAbility`))))