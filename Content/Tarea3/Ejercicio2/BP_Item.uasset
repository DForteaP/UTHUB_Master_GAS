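; BP_Item is a data-driven item actor that applies a gameplay effect to actors overlapping its box.
; The construction script looks up the DT_Items row named after the ItemType enum value, stores it as ItemInfo and shows its name on a text render.
; On overlap, it applies the row's ClassEffect through the other actor's UTHUB_ASC component, if present.
; The item remains in place after applying the effect.
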(event `self.Box.OnComponentBeginOverlap`
  (params (OverlappedComponent :type "PrimitiveComponent Object Reference") (OtherActor :type "Actor Object Reference") (OtherComp :type "PrimitiveComponent Object Reference") (OtherBodyIndex :type Integer) (bFromSweep :type Boolean) (SweepResult :type "HitResult Structure (by ref)"))
  (bind _returnvalue (`self.GetComponentByClass` OtherActor "/Script/UTHUB_GAS.UTHUB_ASC"))
  (bind (_iteminfo_name _iteminfo_classeffect) (break `/Game/Tarea3/Ejercicio2/S_Items` (`self.ItemInfo`)))
  (`/Engine/EditorBlueprintResources/StandardMacros.IsValid` _returnvalue
    (:`Is Valid`
      (`UTHUB_ASC.ApplyGameplayEffect` _returnvalue _iteminfo_classeffect))))

(fn `UserConstructionScript`
  (bind _iteminfo_name (break `/Game/Tarea3/Ejercicio2/S_Items` (`self.ItemInfo`)))
  (bind _returnvalue (`|GetDataTableRow` "/Game/Tarea3/Ejercicio2/DT_Items.DT_Items" (`KismetStringLibrary.Conv_StringToName` (`|GetEnumeratorNameAsString` (`self.ItemType`))))
    (:`then`
      (set `self.ItemInfo` _returnvalue)
      (`TextRenderComponent.K2_SetText` (`self.TextRender`) (`KismetTextLibrary.Conv_NameToText` _iteminfo_name)))))