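; BP_Lava is a lava hazard that applies a damage Gameplay Effect to actors with a UTHUB_ASC inside its box.
; A looping timer reapplies the effect to overlapping actors, passing damage as a SetByCaller magnitude under the LavaDamage tag.
; The PlayerEffects map keeps each actor's latest effect handle, overwritten on every application.
; Leaving the box removes that stored effect and, on success, clears the map entry.
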(event `self.ReceiveBeginPlay`
  (`KismetSystemLibrary.K2_SetTimerDelegate` (delegate `Initeffects`) (`self.Time`) true))

(event `Initeffects`
  (for _array_element (`PrimitiveComponent.GetOverlappingActors` (`self.Box`) null)
    (`self.Apply Damage GE` _array_element)))

(event `self.Box.OnComponentEndOverlap`
  (params (OverlappedComponent :type "PrimitiveComponent Object Reference") (OtherActor :type "Actor Object Reference") (OtherComp :type "PrimitiveComponent Object Reference") (OtherBodyIndex :type Integer))
  (bind (_value _returnvalue) (`BlueprintMapLibrary.Map_Find` (`self.PlayerEffects`) OtherActor))
  (if _returnvalue
    (`self.Remove Damage GE` _value OtherActor)))

(fn `Apply Damage GE`
  (params (TargetActor :type "Actor Object Reference"))
  (bind _returnvalue (`self.GetComponentByClass` TargetActor "/Script/UTHUB_GAS.UTHUB_ASC"))
  (`/Engine/EditorBlueprintResources/StandardMacros.IsValid` _returnvalue
    (:`Is Valid`
      (bind _returnvalue_2 (`AbilitySystemBlueprintLibrary.AssignTagSetByCallerMagnitude` (`AbilitySystemComponent.MakeOutgoingSpec` :`self` _returnvalue :`GameplayEffectClass` (`self.Effect Class`)) (struct :`TagName` "Tarea3.LavaDamage") (`self.Damage`)))
      (bind _returnvalue_3 (`AbilitySystemComponent.BP_ApplyGameplayEffectSpecToTarget` (`self.ASC`) _returnvalue_2 _returnvalue))
      (`BlueprintMapLibrary.Map_Add` (`self.PlayerEffects`) (`local.TargetActor`) _returnvalue_3))))

(fn `Remove Damage GE`
  (params (`Active GameplayEffect` :type "ActiveGameplayEffectHandle Structure") (TargetActor :type "Actor Object Reference"))
  (bind _returnvalue (`self.GetComponentByClass` (`local.TargetActor`) "/Script/UTHUB_GAS.UTHUB_ASC"))
  (`/Engine/EditorBlueprintResources/StandardMacros.IsValid` _returnvalue
    (:`Is Valid`
      (bind _returnvalue_2 (`AbilitySystemComponent.RemoveActiveGameplayEffect` _returnvalue `Active GameplayEffect` -1))
      (if _returnvalue_2
        (`BlueprintMapLibrary.Map_Remove` (`self.PlayerEffects`) (`local.TargetActor`))))))

(fn `UserConstructionScript`)